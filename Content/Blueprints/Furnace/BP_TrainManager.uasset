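; BP_TrainManager initializes BP_Furnace actors with train positions and relays player movement to a furnace.
; On BeginPlay it gives each furnace the PositionsForTrain array and calls SetStartPosition, first inverse-transforming the points when that furnace sits at the world origin.
; It also binds to the player's MovementDirection vector-changed event, forwarding each change to PlayerMovedFunc on the last furnace found.
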(event `self.ReceiveBeginPlay`
  (`|ExecutionSequence`
    (:`then_0`
      (bind _outactors (`GameplayStatics.GetAllActorsOfClass` "/Game/Blueprints/Furnace/BP_Furnace.BP_Furnace_C"))
      (for _array_element _outactors
        (bind _output_get (set `self.AsBP_Furnace` _array_element))
        (if (not (!= (`self.K2_GetActorLocation` _array_element) (0.0 0.0 0.0)))
          (for (_array_element_2 _array_index) (`self.PositionsForTrain`)
            (`KismetArrayLibrary.Array_Set` (`self.PositionsForTrain`) _array_index (`KismetMathLibrary.InverseTransformLocation` (`self.GetTransform` _array_element) _array_element_2))))
        (set `/Game/Blueprints/Furnace/BP_Furnace.PositionsToGoTo` (`self.PositionsForTrain`) _output_get)
        (`/Game/Blueprints/Furnace/BP_Furnace.SetStartPosition` _output_get)))
    (:`then_1`
      (bind _asbp_player (cast `/Game/Blueprints/Characters/Player/BP_Player` (`GameplayStatics.GetPlayerPawn` 0)))
      (bind _output_get_2 (set `self.AsBP_Player` _asbp_player))
      (add `/Game/Blueprints/Components/BPC_VectorCallback.VectorChanged` (`/Game/Blueprints/Characters/Player/BP_Player.MovementDirection` _output_get_2) (delegate `VectorChange`)))))

(event `VectorChange`
  (params (NewLocation :type "Vector Structure"))
  (`/Game/Blueprints/Furnace/BP_Furnace.PlayerMoved_Func` (`self.AsBP_Furnace`) NewLocation (`self.AsBP_Player`)))

(fn `UserConstructionScript`)