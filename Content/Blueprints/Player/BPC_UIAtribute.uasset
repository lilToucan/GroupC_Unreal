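; Player component that stores one attribute as a current and maximum value, named for UI use.
; CurrentValue starts at MaxValue and is clamped between zero and that maximum when changed, while MaxValue cannot drop below MinMaxValue.
; Both changes exist as events and duplicate functions, each broadcasting the requested amount rather than the clamped result.
; Changing MaxValue leaves CurrentValue untouched.
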(event `self.ReceiveBeginPlay`
  (set `self.CurrentValue` (`self.MaxValue`)))

(event `ChangeMaxValueByAmount_Event`
  (params (Amount :type "Float (double-precision)"))
  (set `self.MaxValue` (`KismetMathLibrary.FMax` (+ Amount (`self.MaxValue`)) (`self.MinMaxValue`)))
  (`self.ChangeMaxValueByAmount` Amount))

(event `ChangeValueByAmount_Event`
  (params (Amount :type "Float (double-precision)"))
  (set `self.CurrentValue` (`KismetMathLibrary.FMax` (`KismetMathLibrary.FMin` (+ Amount (`self.CurrentValue`)) (`self.MaxValue`))))
  (`self.ChangeValueByAmount` Amount))

(fn `ChangeMaxValueByAmount_Func`
  (params (Amount :type "Float (double-precision)"))
  (set `self.MaxValue` (`KismetMathLibrary.FMax` (+ Amount (`self.MaxValue`)) (`self.MinMaxValue`)))
  (`self.ChangeMaxValueByAmount` Amount))

(fn `ChangeValueByAmount_Func`
  (params (Amount :type "Float (double-precision)"))
  (set `self.CurrentValue` (`KismetMathLibrary.FMax` (`KismetMathLibrary.FMin` (+ Amount (`self.CurrentValue`)) (`self.MaxValue`))))
  (`self.ChangeValueByAmount` Amount))