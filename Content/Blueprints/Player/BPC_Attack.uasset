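; Player attack component that tracks a combo counter and selects the animation for each successive attack.
; PerformCombo sets IsAttacking, wraps the counter past the end of Animations, fires PerformAttack and returns the matching animation.
; PerformAttack broadcasts and increments the counter, using a retriggerable delay to reset the combo when attacks stop.
; ResetMovement clears IsAttacking, and both resets notify listeners through dispatchers.
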(event `Reset AttackCombo`
  (set `self.AttackCombo` 0)
  (`self.ComboReseted`))

(event `PerformAttack`
  (`self.AttackPerformed`)
  (`/Engine/EditorBlueprintResources/StandardMacros.IncrementInt` (`self.AttackCombo`)
    (:`  `
      (`KismetSystemLibrary.RetriggerableDelay` (`self.ResetComboTimer`))
      (`self.Reset AttackCombo`))))

(event `ResetMovement`
  (set `self.IsAttacking` false)
  (`self.MovementReset`))

(fn `PerformCombo`
  (returns (Animation :type "AnimMontage Object Reference"))
  (locals (NewLocalVar :type Integer :default 0) (NewLocalVar_0 :type Integer :default 0))
  (set `self.IsAttacking` true)
  (if (> (`self.AttackCombo`) (- (`KismetArrayLibrary.Array_Length` (`self.Animations`)) 1))
    (`self.Reset AttackCombo`)
    (`self.PerformAttack`)
    (else
      (`self.PerformAttack`)))
  (return (`|GetArrayItem` (`self.Animations`) (- (`self.AttackCombo`) 1))))