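; BPC_Freeze is a component that tracks a freeze value, which rises while activated and drains back to zero when deactivated.
; ActivateTick and DeactivateTick flip the fill direction and raise activated or deactivated callbacks.
; Tick integrates the value at FillPowerPerSecond and broadcasts it, with no upper clamp.
; Falling below zero resets the value and disables ticking without a final value broadcast.
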(event `self.ReceiveBeginPlay`
  (`self.DeactivateTick`)
  (set `self.CurrentValue` 0.0))

(event `self.ReceiveTick`
  (params (DeltaSeconds :type "Float (single-precision)"))
  (bind _output_get (set `self.CurrentValue` (+ (* DeltaSeconds (`self.FillPowerPerSecond`) (`self.Direction`)) (`self.CurrentValue`))))
  (if (> 0.0 _output_get)
    (set `self.CurrentValue` 0.0)
    (`self.SetComponentTickEnabled` false)
    (else
      (`self.OnValueChanged` (`self.CurrentValue`)))))

(fn `ActivateTick`
  (set `self.Direction` 1.0)
  (`self.OnActivated`)
  (`self.SetComponentTickEnabled` true))

(fn `DeactivateTick`
  (set `self.Direction` -1.0)
  (`self.OnDeactivated`))