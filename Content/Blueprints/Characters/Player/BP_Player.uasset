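; Player character Blueprint with camera-relative movement, stamina-limited running, cursor-aimed pickaxe attacks and a HUD.
; BeginPlay wires up the pickaxe child actor's combo animations and attack reset; while attacking, Tick turns the player toward the cursor hit point instead of movement direction.
; Health and stamina components handle damage and run drain/regen, with depleted health or a filled FreezeTick calling an empty Die.
; Interaction, slot-scrolling and crossbow logic remain as disconnected leftovers.
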(event `self.ReceiveBeginPlay`
  (`|ExecutionSequence`
    (:`then_0`
      (bind _asbp_pickaxe (cast `/Game/Blueprints/Weapons/BP_Pickaxe` (`ChildActorComponent.ChildActor` (`self.BP_Pickaxe_`))))
      (bind _output_get (set `self.As BP Pickaxe` _asbp_pickaxe))
      (set `/Game/Blueprints/Weapons/BP_Pickaxe.PickaxeOwner` self _output_get)
      (set `/Game/Blueprints/Weapons/BPC_Attack.Animations` (`self.ComboAnimations`) (`/Game/Blueprints/Weapons/BP_Pickaxe.Combo` (`self.As BP Pickaxe`))))
    (:`then_1`
      (set `self.NormalMoveSpeed` (`MovementComponent.GetMaxSpeed` (`self.CharacterMovement`)))
      (bind _returnvalue (`|CreateWidget` "/Game/UI/WBP_UI.WBP_UI_C" (`GameplayStatics.GetPlayerController` 0)))
      (bind _output_get_2 (set `self.PlayerHUD` _returnvalue))
      (`UserWidget.AddToViewport` _output_get_2 0))
    (:`then_2`
      (add `/Game/Blueprints/Weapons/BPC_Attack.MovementReset` (`/Game/Blueprints/Weapons/BP_Pickaxe.Combo` (`self.As BP Pickaxe`)) (delegate `ResetAttackInput`))
      (set `PlayerController.bShowMouseCursor` true (`GameplayStatics.GetPlayerController` 0)))))

(event `self.ReceiveAnyDamage`
  (params (Damage :type "Float (single-precision)") (DamageType :type "DamageType Object Reference") (InstigatedBy :type "Controller Object Reference") (DamageCauser :type "Actor Object Reference"))
  (`/Game/Blueprints/Components/BPC_UIAtribute.ChangeValueByAmount_Func` (`self.Healt`) (* Damage -1.0)))

(event `ResetAttackInput`
  (set `self.IsAttacking` false))

(event `self.Healt.ChangeValueByAmount`
  (params (Amount :type "Float (double-precision)"))
  (if (<= (`/Game/Blueprints/Components/BPC_UIAtribute.CurrentValue` (`self.Healt`)) 0.0)
    (`self.Die`)))

(event `self.ReceiveTick`
  (params (DeltaSeconds :type "Float (single-precision)"))
  ;[0 0.9479 0.2261 0.5] Running Stamina Depleation
  (`self.CheckStamina` DeltaSeconds)
  (if (`self.IsAttacking`)
    (`self.SetRotationToLookDir`)
    (`self.SetDirection`)
    (else
      (set `CharacterMovementComponent.bOrientRotationToMovement` true (`self.CharacterMovement`)))))

(event `Die`)

(event `EnhancedInput|/Game/Inputs/Actions/Movement/IA_Movement`
  (params (ActionValue :type "Vector2D Structure") (ElapsedSeconds :type "Float (double-precision)") (TriggeredSeconds :type "Float (double-precision)") (InputAction :type "InputAction Object Reference" :default "/Game/Inputs/Actions/Movement/IA_Movement.IA_Movement"))
  (bind (_returnvalue_roll _returnvalue_pitch _returnvalue_yaw) (`KismetMathLibrary.BreakRotator` (`self.GetControlRotation`)))
  ;[0 0 0 0.5 122] Inputs
  ;;[0.0432 0.15 0.1134 0.5] Movement
  (:`Triggered`
    (set `self.IsMoving` true)
    (bind _output_get (set `self.moveDirection` (`KismetMathLibrary.Normal` (`KismetMathLibrary.GreaterGreater_VectorRotator` (`KismetMathLibrary.MakeVector` ActionValue_X ActionValue_Y) (`KismetMathLibrary.MakeRotator` 0.0 0.0 _returnvalue_yaw)))))
    (`self.AddMovementInput` _output_get))
  (:`Completed`
    (set `self.IsMoving` false)
    (`/Game/Blueprints/Components/BPC_VectorCallback.ChangeVector` (`self.MovementDirection`) (0.0 0.0 0.0))
    (set `self.IsRunning` false)))

(event `EnhancedInput|/Game/Inputs/Actions/Movement/IA_Run`
  (params (ActionValue :type Boolean) (ElapsedSeconds :type "Float (double-precision)") (TriggeredSeconds :type "Float (double-precision)") (InputAction :type "InputAction Object Reference" :default "/Game/Inputs/Actions/Movement/IA_Run.IA_Run"))
  ;[0 0 0 0.5 122] Inputs
  ;;[0 1 0.4034 0.5] Run
  (:`Started`
    (if (and (not (`self.IsRunning`)) (`self.IsMoving`))
      (set `CharacterMovementComponent.MaxWalkSpeed` (`self.RunSpeed`) (`self.CharacterMovement`))
      (set `self.IsRunning` true)
      (else
        (set `CharacterMovementComponent.MaxWalkSpeed` (`self.NormalMoveSpeed`) (`self.CharacterMovement`))
        (set `self.IsRunning` false)))))

(event `EnhancedInput|/Game/Inputs/Actions/Combat/IA_AttackInput`
  (params (ActionValue :type Boolean) (ElapsedSeconds :type "Float (double-precision)") (TriggeredSeconds :type "Float (double-precision)") (InputAction :type "InputAction Object Reference" :default "/Game/Inputs/Actions/Combat/IA_AttackInput.IA_AttackInput"))
  ;[0 0 0 0.5 122] Inputs
  ;;[0.2708 0.749 0.8385 0.5] Pickaxe
  (:`Started`
    (if (not (`self.IsAttacking`))
      (set `self.IsAttacking` true)
      (`/Game/Blueprints/Weapons/BP_Pickaxe.Use` (`self.As BP Pickaxe`) null)
      ;; Set Running to false
      (set `self.IsRunning` false)
      (`self.SetAimPos`))))

(event `EnhancedInput|/Game/Inputs/Actions/Combat/IA_ShootArrow`
  (params (ActionValue :type Boolean) (ElapsedSeconds :type "Float (double-precision)") (TriggeredSeconds :type "Float (double-precision)") (InputAction :type "InputAction Object Reference" :default "/Game/Inputs/Actions/Combat/IA_ShootArrow.IA_ShootArrow"))
  ;[0 0 0 0.5 122] Inputs
  (:`Canceled`
    (set `self.IsAttacking` false)))

(event `EnhancedInput|/Game/Inputs/Actions/Interactions/IA_Grab`
  (params (ActionValue :type Boolean) (ElapsedSeconds :type "Float (double-precision)") (TriggeredSeconds :type "Float (double-precision)") (InputAction :type "InputAction Object Reference" :default "/Game/Inputs/Actions/Interactions/IA_Grab.IA_Grab"))
  ;[0 0 0 0.5 122] Inputs
  ;; Disconnect, now in BP_InventoryComponent
)

(event `/Game/Blueprints/Characters/BaseClass/BPI_Entity.AttackOverlapSphere`
  (bind _returnvalue (`SceneComponent.K2_GetComponentLocation` (`self.BP_Pickaxe_`)))
  ;[0 0 0 0.5] Attack Collision
  (`KismetSystemLibrary.DrawDebugSphere` _returnvalue 10.0 12 (struct :`R` 1.0 :`G` 0.340781 :`B` 0.686097 :`A` 1.0) 10.0 0.5)
  (bind _outactors (`KismetSystemLibrary.SphereOverlapActors` _returnvalue 10.0 (`|MakeArray` "ObjectTypeQuery7" "ObjectTypeQuery1" :!type "EObjectTypeQuery Enum")))
  (for _array_element _outactors
    (`GameplayStatics.ApplyDamage` _array_element (`/Game/Blueprints/Weapons/BP_Pickaxe.DamageValue` (`self.As BP Pickaxe`)) (`self.GetController`) self)))

(event `EnhancedInput|/Game/Inputs/Actions/Inventory/IA_MouseScrollUp`
  (params (ActionValue :type Boolean) (ElapsedSeconds :type "Float (double-precision)") (TriggeredSeconds :type "Float (double-precision)") (InputAction :type "InputAction Object Reference" :default "/Game/Inputs/Actions/Inventory/IA_MouseScrollUp.IA_MouseScrollUp"))
  ;[0 0 0 0.5 122] Inputs
  ;;[0 0 0 0.5 100] Inventory Inputs
)

(event `EnhancedInput|/Game/Inputs/Actions/Inventory/IA_MouseScrollDown`
  (params (ActionValue :type Boolean) (ElapsedSeconds :type "Float (double-precision)") (TriggeredSeconds :type "Float (double-precision)") (InputAction :type "InputAction Object Reference" :default "/Game/Inputs/Actions/Inventory/IA_MouseScrollDown.IA_MouseScrollDown"))
  ;[0 0 0 0.5 122] Inputs
  ;;[0 0 0 0.5 100] Inventory Inputs
)

(event `SetAimPos`
  (bind (_returnvalue_x _returnvalue_y _returnvalue_z) (`KismetMathLibrary.BreakVector` (`self.K2_GetActorLocation`)))
  (bind (_bblockinghit _binitialoverlap _time _distance _location _impactpoint) (`GameplayStatics.BreakHitResult` (`PlayerController.GetHitResultUnderCursorByChannel` (`GameplayStatics.GetPlayerController` 0) "TraceTypeQuery1" true)))
  (set `self.AimTargetPos` (`KismetMathLibrary.MakeVector` (.x _impactpoint) (.y _impactpoint) _returnvalue_z))
  (set `CharacterMovementComponent.bOrientRotationToMovement` false (`self.CharacterMovement`)))

(event `Key|AnyKey`
  (params (Key :type "Key Structure"))
  ;[0 0 0 0.5 122] Inputs
  ;;[0 0 0 0.5 100] Inventory Inputs
)

(event `Shoot`
  (bind _mesh (`self.Mesh`))
  (`|SpawnActorFromClass` "/Game/Blueprints/Weapons/BP_Arrow.BP_Arrow_C" (`KismetMathLibrary.MakeTransform` (`SceneComponent.GetSocketLocation` _mesh (`SkinnedMeshComponent.GetSocketBoneName` _mesh "ArrowSocket")) (`KismetMathLibrary.FindLookAtRotation` (0.0 0.0 0.0) (`KismetMathLibrary.Vector_Forward`))) "Undefined" "MultiplyWithRoot" null null))

(event `SetRotationToLookDir`
  (bind (_returnvalue_roll _returnvalue_pitch) (`KismetMathLibrary.BreakRotator` (`self.K2_GetActorRotation`)))
  (bind (_returnvalue_roll_2 _returnvalue_pitch_2 _returnvalue_yaw) (`KismetMathLibrary.BreakRotator` (`KismetMathLibrary.FindLookAtRotation` (`KismetMathLibrary.Vector_Zero`) (- (`self.AimTargetPos`) (`self.K2_GetActorLocation`)))))
  (`self.K2_SetActorRotation` (`KismetMathLibrary.MakeRotator` _returnvalue_roll _returnvalue_pitch _returnvalue_yaw)))

(event `Reload`)

(event `SetDirection`
  (set `self.DirectionAngle` (/ (`KismetMathLibrary.Acos` (`KismetMathLibrary.Dot_VectorVector` (`self.moveDirection`) (`self.GetActorForwardVector` self))) 180.0)))

(event `self.FreezeTick.OnValueChanged`
  (params (Value :type "Float (double-precision)"))
  (if (>= Value (`/Game/Blueprints/Components/BPC_Freeze.FilledValue` (`self.FreezeTick`)))
    (`self.Die`)
    (`/Game/Blueprints/Components/BPC_Freeze.DeactivateTick` (`self.FreezeTick`))
    (else
      ; Recharge it
      (`/Game/Blueprints/Components/BPC_Freeze.DeactivateTick` (`self.FreezeTick`)))))

(event `/Game/Blueprints/Characters/BaseClass/BPI_Entity.AfterUsingItem`
  (set `self.IUsable` null))

(fn `CheckStamina`
  (params (DeltaTime :type "Float (double-precision)"))
  (bind _stamina (`self.Stamina`))
  (if (`self.IsRunning`)
    (`self.SubtractStamina` DeltaTime)
    (set `CharacterMovementComponent.MaxWalkSpeed` (`self.RunSpeed`) (`self.CharacterMovement`))
    (elif (< (`/Game/Blueprints/Components/BPC_UIAtribute.CurrentValue` _stamina) (`/Game/Blueprints/Components/BPC_UIAtribute.MaxValue` _stamina))
      (`self.RegenStamina` DeltaTime)
      (set `CharacterMovementComponent.MaxWalkSpeed` (`self.NormalMoveSpeed`) (`self.CharacterMovement`)))))

(fn `ItemOverlapSphere`
  (returns (HitObjects :type "Array of Actor Object Reference"))
  (bind _returnvalue (+ (`self.K2_GetActorLocation`) (* (`self.GetActorForwardVector`) 100.0)))
  (bind _outactors (`KismetSystemLibrary.SphereOverlapActors` _returnvalue 100.0 (`|MakeArray` "ObjectTypeQuery1" "ObjectTypeQuery2" :!type "EObjectTypeQuery Enum")))
  (`KismetSystemLibrary.DrawDebugSphere` _returnvalue 100.0 12 (struct :`R` 1.0 :`G` 1.0 :`B` 1.0 :`A` 1.0) 10.0)
  (return _outactors))

(fn `OverlapSphere`
  (`KismetSystemLibrary.SphereTraceSingle` :`End` (- (`self.K2_GetActorLocation`) (0.0 0.0 65.0)) :`Radius` (`self.InteractionRadious`) :`TraceChannel` "TraceTypeQuery1" :`DrawDebugType` "ForDuration")
  (for _array_element _
    (bind _asbpi_usable (cast `/Game/Blueprints/Weapons/BPI_Usable` _array_element))
    (set `self.IUsable` _asbpi_usable)
    (`KismetSystemLibrary.DrawDebugSphere` (`self.K2_GetActorLocation`) (`self.InteractionRadious`) 12 (struct :`R` 1.0 :`G` 1.0 :`B` 1.0 :`A` 1.0) 10.0)
    (break)))

(fn `RealoadFunction`
  (params (TimePassed :type "Float (double-precision)"))
  (returns (NewParam :type Boolean))
  (return (> TimePassed 0.0)))

(fn `RegenStamina`
  (params (DeltaTime :type "Float (double-precision)"))
  (`/Game/Blueprints/Components/BPC_UIAtribute.ChangeValueByAmount_Func` (`self.Stamina`) (* (`self.StaminaRegenPerSecond`) DeltaTime)))

(fn `SubtractStamina`
  (params (DeltaTime :type "Float (double-precision)"))
  (`/Game/Blueprints/Components/BPC_UIAtribute.ChangeValueByAmount_Func` (`self.Stamina`) (* (* DeltaTime (`self.StaminaUsedPerSecond`)) -1.0))
  (if (<= (`/Game/Blueprints/Components/BPC_UIAtribute.CurrentValue` (`self.Stamina`)) 0.0)
    (set `CharacterMovementComponent.MaxWalkSpeed` (`self.NormalMoveSpeed`) (`self.CharacterMovement`))
    (set `self.IsRunning` false)))

(fn `UserConstructionScript`)