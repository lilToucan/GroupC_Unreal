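; BP_ArrowProjectile is an arrow projectile that damages actors it overlaps.
; Overlaps with its Parent are ignored; any other overlap destroys the arrow, applying Damage first unless the actor's class is BP_Furnace.
; Tick also destroys the arrow once it is beyond a fixed distance from the Parent's current location, rather than from its spawn point.
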(event `self.ReceiveTick`
  (params (DeltaSeconds :type "Float (single-precision)"))
  (if (> (`KismetMathLibrary.Vector_Distance` (`self.K2_GetActorLocation` (`self.Parent`)) (`self.K2_GetActorLocation`)) 10000.0)
    (`self.K2_DestroyActor`)))

(event `self.ReceiveActorBeginOverlap`
  (params (OtherActor :type "Actor Object Reference"))
  (`self.OnOverlap` OtherActor))

(fn `OnOverlap`
  (params (InputPin :type "Actor Object Reference"))
  (if (not (== (`local.InputPin`) (`self.Parent`)))
    (if (not (== (`GameplayStatics.GetObjectClass` (`local.InputPin`)) "/Game/Blueprints/Furnace/BP_Furnace.BP_Furnace_C"))
      (`GameplayStatics.ApplyDamage` (`local.InputPin`) (`self.Damage`)))
    (`self.K2_DestroyActor`)))

(fn `UserConstructionScript`)