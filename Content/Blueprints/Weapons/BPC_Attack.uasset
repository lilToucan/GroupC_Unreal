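; BPC_Attack is an attack combo component that tracks the current combo step and supplies the matching attack animation.
; PerformCombo wraps the counter after the last entry in Animations, triggers PerformAttack and returns that step's animation.
; Each attack fires AttackPerformed, advances the counter and restarts a retriggerable delay that resets the combo when it expires.
; Combo and movement resets are broadcast through ComboReseted and MovementReset calls.
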(event `Reset AttackCombo`
  (set `self.AttackCombo` 0)
  (`self.ComboReseted`))

(event `PerformAttack`
  (`self.AttackPerformed`)
  (`/Engine/EditorBlueprintResources/StandardMacros.IncrementInt` (`self.AttackCombo`)
    (:`  `
      (`KismetSystemLibrary.RetriggerableDelay` (`self.ResetComboTimer`))
      (`self.Reset AttackCombo`))))

(event `ResetMovement`
  (`self.MovementReset`))

(fn `PerformCombo`
  (returns (Animation :type "AnimMontage Object Reference"))
  (locals (NewLocalVar :type Integer :default 0) (NewLocalVar_0 :type Integer :default 0))
  (if (> (`self.AttackCombo`) (- (`KismetArrayLibrary.Array_Length` (`self.Animations`)) 1))
    (`self.Reset AttackCombo`)
    (`self.PerformAttack`)
    (else
      (`self.PerformAttack`)))
  (return (`|GetArrayItem` (`self.Animations`) (- (`self.AttackCombo`) 1))))