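; Interactable inventory station that holds items in its own inventory component and transfers them to and from the interacting inventory.
; The first interaction activates it; later ones hand over the current or next filled slot, closing if both are empty.
; Primary item use while active deposits into the station with stacking, while non-primary use closes it.
; Stored item actors are hidden without collision, then restored at the station's location when dropped.
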(event `self.BPC_Inventory.OnPickUpItem`
  (params (PickedUpItem :type "/Game/Blueprints/Characters/Struct/S_Items Structure") (ItemSlot :type Integer))
  (`self.SetActorHiddenInGame` PickedUpItem_ItemActor_22_19FB7DB04A84A2155A9BE29059FD9CD6 true)
  (`self.SetActorEnableCollision` PickedUpItem_ItemActor_22_19FB7DB04A84A2155A9BE29059FD9CD6 false))

(event `self.BPC_Inventory.OnDropItem`
  (params (DropedItem :type "/Game/Blueprints/Characters/Struct/S_Items Structure") (ItemSlot :type Integer))
  (bind (_name _isstackable _quantity _thumbnail _staticmesh _itemactor) (break `/Game/Blueprints/Characters/Struct/S_Items` DropedItem))
  (`/Engine/EditorBlueprintResources/StandardMacros.IsValid` _itemactor
    (:`Is Valid`
      (`self.K2_SetActorLocation` _itemactor (`self.K2_GetActorLocation`) false false)
      (`self.SetActorHiddenInGame` _itemactor false)
      (`self.SetActorEnableCollision` _itemactor true))))

(fn `Close`
  (`parent.Close`))

(fn `DropItem`
  (params (Item :type "/Game/Blueprints/Characters/Struct/S_Items Structure")))

(fn `InteractFunction`
  (params (inventoryInteracted :type "/Game/UI/Inventory_UI/BPC_Inventory Object Reference"))
  (if (`self.IsActive`)
    ; Is the current slot filled?
    (bind _itemref (`/Game/UI/Inventory_UI/BPC_Inventory.GetCurrentSlot` (`self.BPC_Inventory`)))
    (if (> (`.Quantity_8_1C15349B4EEFEF5AD272EF8EB4F779DF` (break `/Game/Blueprints/Characters/Struct/S_Items` _itemref)) 0)
      (`/Game/UI/Inventory_UI/BPC_Inventory.Transfer` (`local.inventoryInteracted`) (`self.BPC_Inventory`) false)
      (else
        ; Is the next one filled?
        (`/Game/UI/Inventory_UI/BPC_Inventory.ChangeSlot` (`self.BPC_Inventory`) 1)
        (bind _itemref_2 (`/Game/UI/Inventory_UI/BPC_Inventory.GetCurrentSlot` (`self.BPC_Inventory`)))
        (if (> (`.Quantity_8_1C15349B4EEFEF5AD272EF8EB4F779DF` (break `/Game/Blueprints/Characters/Struct/S_Items` _itemref_2)) 0)
          (`/Game/UI/Inventory_UI/BPC_Inventory.Transfer` (`local.inventoryInteracted`) (`self.BPC_Inventory`) false)
          (else
            (`self.Close`)))))
    (else
      (`self.OnInteraction`)
      (set `self.IsActive` true))))

(fn `ItemInteraction`
  (params (Item :type "/Game/Blueprints/Test/Items/BP_Item Object Reference") (InventoryCalled :type "/Game/UI/Inventory_UI/BPC_Inventory Object Reference") (IsPrimary :type Boolean))
  (if (`self.IsActive`)
    (if (`local.IsPrimary`)
      (bind _output_get (set `self.OldInventory` (`local.InventoryCalled`)))
      (`/Game/UI/Inventory_UI/BPC_Inventory.Transfer` (`self.BPC_Inventory`) _output_get true)
      (else
        (`self.Close`)))
    (else
      (`self.InteractFunction` InventoryCalled))))

(fn `PickUpFunction`
  (params (Item :type "/Game/Blueprints/Characters/Struct/S_Items Structure"))
  (`/Engine/EditorBlueprintResources/StandardMacros.IsValid` Item_ItemActor_22_19FB7DB04A84A2155A9BE29059FD9CD6
    (:`Is Valid`
      (`/Game/UI/Inventory_UI/BPC_Inventory.OnPickupFunction` (`self.BPC_Inventory`) Item_ItemActor_22_19FB7DB04A84A2155A9BE29059FD9CD6))))

(fn `UserConstructionScript`)