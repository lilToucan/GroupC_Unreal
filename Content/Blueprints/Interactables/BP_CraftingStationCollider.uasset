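; BP_CraftingStationCollider is an interactable crafting station that inherits its construction logic from a parent class.
; InteractFunction toggles it: an active station closes, while an inactive one calls its interaction notification and becomes active.
; While active, ItemInteraction hands the station and calling inventory to the item's Craft or SecondaryCraft, depending on the primary flag, so items handle the crafting themselves.
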(fn `InteractFunction`
  (params (inventoryInteracted :type "/Game/UI/Inventory_UI/BPC_Inventory Object Reference"))
  (if (`self.IsActive`)
    (`self.Close`)
    (else
      (`self.OnInteraction`)
      (set `self.IsActive` true))))

(fn `ItemInteraction`
  (params (Item :type "/Game/Blueprints/Test/Items/BP_Item Object Reference") (InventoryCalled :type "/Game/UI/Inventory_UI/BPC_Inventory Object Reference") (IsPrimary :type Boolean))
  (if (`self.IsActive`)
    (if (`local.IsPrimary`)
      (`/Game/Blueprints/Test/Items/BP_Item.Craft` (`local.Item`) self (`local.InventoryCalled`))
      (else
        (`/Game/Blueprints/Test/Items/BP_Item.SecondaryCraft` (`local.Item`) self (`local.InventoryCalled`))))))

(fn `UserConstructionScript`
  (`parent.UserConstructionScript`))