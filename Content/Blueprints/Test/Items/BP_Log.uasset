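; BP_Log is a log inventory item that serves as furnace fuel and as a crafting material.
; Use recharges the furnace's fuel velocity and SecondaryUse recharges its fuel heat, both by the same recharge amount.
; Craft spawns BP_Coal and SecondaryCraft spawns BP_Arrow at the interactable's location.
; All four actions then call UsedItem on the inventory's current slot, while startup and construction defer to the parent class.
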(event `self.ReceiveBeginPlay`
  (`self.StartUp`))

(fn `Craft`
  (params (Interactable :type "/Game/Blueprints/Interactables/BP_interactable Object Reference") (Inventory :type "/Game/UI/Inventory_UI/BPC_Inventory Object Reference"))
  (bind _returnvalue_location (`KismetMathLibrary.BreakTransform` (`self.GetTransform` Interactable)))
  (`|SpawnActorFromClass` "/Game/Blueprints/Test/Items/BP_Coal.BP_Coal_C" (`KismetMathLibrary.MakeTransform` _returnvalue_location) "Undefined" "MultiplyWithRoot" null null)
  (`self.CallUsedItem` (`local.Inventory`) (`/Game/UI/Inventory_UI/BPC_Inventory.CurrentSlot` (`local.Inventory`))))

(fn `SecondaryCraft`
  (params (Interactable :type "/Game/Blueprints/Interactables/BP_interactable Object Reference") (Inventory :type "/Game/UI/Inventory_UI/BPC_Inventory Object Reference"))
  (bind _returnvalue_location (`KismetMathLibrary.BreakTransform` (`self.GetTransform` Interactable)))
  (`|SpawnActorFromClass` "/Game/Blueprints/Test/Items/BP_Arrow.BP_Arrow_C" (`KismetMathLibrary.MakeTransform` _returnvalue_location) "Undefined" "MultiplyWithRoot" null null)
  (`self.CallUsedItem` (`local.Inventory`) (`/Game/UI/Inventory_UI/BPC_Inventory.CurrentSlot` (`local.Inventory`))))

(fn `SecondaryUse`
  (params (Inventory :type "/Game/UI/Inventory_UI/BPC_Inventory Object Reference") (Furnace :type "/Game/Blueprints/Furnace/BP_Furnace Object Reference"))
  (`/Game/Blueprints/Furnace/BP_Furnace.RechargeFuelHeat` Furnace (`self.FuelRechargeAmount`))
  (`self.CallUsedItem` (`local.Inventory`) (`/Game/UI/Inventory_UI/BPC_Inventory.CurrentSlot` (`local.Inventory`))))

(fn `StartUp`
  (`parent.StartUp`))

(fn `Use`
  (params (Inventory :type "/Game/UI/Inventory_UI/BPC_Inventory Object Reference") (Frunace :type "/Game/Blueprints/Furnace/BP_Furnace Object Reference"))
  (`/Game/Blueprints/Furnace/BP_Furnace.RechargeFuelVelocity` Frunace (`self.FuelRechargeAmount`))
  (`self.CallUsedItem` (`local.Inventory`) (`/Game/UI/Inventory_UI/BPC_Inventory.CurrentSlot` (`local.Inventory`))))

(fn `UserConstructionScript`
  (`parent.UserConstructionScript`))